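; BP_BallKickController spawns a ball at the player character for a kick action.
; Its Kick function destroys the previous ball if still valid, spawns a new one slightly ahead of player 0's character along its forward vector, and stores it as LastBall.
; This keeps one ball from this controller at a time; the function applies no impulse, and BeginPlay and Tick are unused.
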(fn `kick`
  (bind _returnvalue (`GameplayStatics.GetPlayerCharacter` 0))
  (bind _lastball (`self.lastBall`))
  ;[1 1 1] Spawn Ball
  (if (`KismetSystemLibrary.IsValid` _lastball)
    (`Actor.K2_DestroyActor` _lastball))
  (bind _returnvalue_2 (`|SpawnActorFromClass` "/Game/Blueprints/BP_Ball.BP_Ball_C" (`KismetMathLibrary.Conv_VectorToTransform` (+ (`Actor.K2_GetActorLocation` _returnvalue) (* (`Actor.GetActorForwardVector` _returnvalue) 20.0))) "Undefined" "MultiplyWithRoot" null null))
  (set `self.lastBall` _returnvalue_2))