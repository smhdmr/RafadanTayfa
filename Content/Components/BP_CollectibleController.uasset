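; Collectible controller that tracks which items have been collected and signals progress to the rest of the game.
; CollectItem flags the given index in a boolean array, fires the item-collected dispatcher and increments the current item index.
; It then scans the array, stopping at the first uncollected entry, and fires the all-items-collected dispatcher when none remain.
; Both steps print on-screen messages, and the event graph holds no active logic.
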(fn `collectItem`
  (params (itemIndex :type Integer))
  ;[1 1 1] Collect Item
  (`KismetArrayLibrary.Array_Set` (`self.isItemCollected`) itemIndex true)
  (`self.onItemCollected`)
  (set `self.currentItemIndex` (+ (`self.currentItemIndex`) 1))
  (`KismetSystemLibrary.PrintString` "Item Collected" true true (struct :`G` 0.66 :`B` 1.0 :`A` 1.0) 10.0)
  ;[1 1 1] Check All Items Collected
  (set `self.isAllItemsCollected` true)
  (for _array_element (`self.isItemCollected`)
    (if (not _array_element)
      (set `self.isAllItemsCollected` false)
      (break)))
  (if (`self.isAllItemsCollected`)
    (`self.onAllItemsCollected`)
    (`KismetSystemLibrary.PrintString` "All Items Collected" true true (struct :`G` 0.66 :`B` 1.0 :`A` 1.0) 10.0)))